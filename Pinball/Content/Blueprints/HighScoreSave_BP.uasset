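; High score save Blueprint that holds a short, ranked list of score structs.
; AddHighScore appends a new entry, sorts the list from highest to lowest, then trims it to at most four.
; SortSavedData is a selection sort that repeatedly moves the highest entry into a temporary array and copies that back.
; A lowest-score lookup is also provided but is not called by the other functions here.
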(fn DetermineLowestValueScore
  ;[1 1 1] Find the lowest index of the lowest score and set it to both var
  (for (_array_element _array_index) (Variables|Default|GetSaveStruct)
    (LocalVariables|SetArray%20Element%20Score (.score _array_element))
    (LocalVariables|SetArray%20Index _array_index)
    (if (== (LocalVariables|GetArray%20Index) 0)
      (LocalVariables|SetLowest%20Score (LocalVariables|GetArray%20Element%20Score))
      (LocalVariables|SetLowest%20Index (LocalVariables|GetArray%20Index))
      (elif (< (LocalVariables|GetArray%20Element%20Score) (LocalVariables|GetLowest%20Score))
        (LocalVariables|SetLowest%20Score (LocalVariables|GetArray%20Element%20Score))
        (LocalVariables|SetLowest%20Index (LocalVariables|GetArray%20Index)))))
  (return (Utilities|Array|Get(acopy) (Variables|Default|GetSaveStruct) (LocalVariables|GetLowest%20Index)) (LocalVariables|GetLowest%20Index)))

(fn DetermineHighestValueScore
  ;[1 1 1] Find the highest index of the highest score and set it to both var
  (for (_array_element _array_index) (Variables|Default|GetSaveStruct)
    (LocalVariables|SetArray%20Element%20Score (.score _array_element))
    (LocalVariables|SetArray%20Index _array_index)
    (if (== (LocalVariables|GetArray%20Index) 0)
      (LocalVariables|SetHighest%20Score (LocalVariables|GetArray%20Element%20Score))
      (LocalVariables|SetHighest%20Index (LocalVariables|GetArray%20Index))
      (elif (> (LocalVariables|GetArray%20Element%20Score) (LocalVariables|GetHighest%20Score))
        (LocalVariables|SetHighest%20Score (LocalVariables|GetArray%20Element%20Score))
        (LocalVariables|SetHighest%20Index (LocalVariables|GetArray%20Index)))))
  (return (Utilities|Array|Get(acopy) (Variables|Default|GetSaveStruct) (LocalVariables|GetHighest%20Index)) (LocalVariables|GetHighest%20Index)))

(fn SortSavedData
  (while (> (Utilities|Array|Length (Variables|Default|GetSaveStruct)) 0)
    (bind (_highest_score_struct _highest_score_index) (CallFunction|DetermineHighestValueScore))
    (Utilities|Array|Add (LocalVariables|GetTempSaveStruct) _highest_score_struct)
    (Utilities|Array|RemoveIndex (Variables|Default|GetSaveStruct) _highest_score_index))
  (Variables|Default|SetSaveStruct (LocalVariables|GetTempSaveStruct)))

(fn AddHighScore
  (params (New%20Score :type High%20Score%20Struct%20BP%20Structure))
  (bind _savestruct (Variables|Default|GetSaveStruct))
  (Utilities|Array|Add (Variables|Default|GetSaveStruct) New%20Score)
  (CallFunction|SortSavedData)
  (Utilities|Array|Resize _savestruct (Math|Integer|Min(Integer) 4 (Utilities|Array|Length _savestruct))))