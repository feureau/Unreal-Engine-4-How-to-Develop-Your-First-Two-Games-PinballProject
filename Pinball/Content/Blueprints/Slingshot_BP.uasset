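; Slingshot bumper actor that kicks the ball away and awards score when the ball overlaps it.
; On overlap with BallSphere_BP, it applies a strong impulse along the capsule's forward vector and restarts a timeline.
; The timeline drives "Percent Out" on a dynamic material, created in the construction script, to animate the band snap.
; Points go to GameMode_BP on every timeline update, rather than once per hit.
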(event EventBeginPlay)

(event Collision|EventActorBeginOverlap
  (params (OtherActor :type Actor%20Object%20Reference))
  ;[1 1 1] Bounce the ball away using impulse - forward vector and multiplier
  (bind _asball_sphere_bp (Utilities|Casting|CastToBallSphere_BP OtherActor))
  (Physics|AddImpulse (Variables|/Game/Blueprints/BallSphere_BP.BallSphere_BP_C|GetBallSphere _asball_sphere_bp) (* (Math|Vector|GetForwardVector (Variables|Default|GetCapsule)) 2e+06) "None" false)
  ;[1 1 1] Timeline control the morphband material's Percent Out to animate the band snaps
  (bind _bounce (Timeline|SlingBounce_Timeline PlayFromStart)
    (:Update
      (bind _asmaterial_instance_dynamic (Utilities|Casting|CastToMaterialInstanceDynamic (Rendering|Material|GetMaterial (Variables|Default|GetStaticMesh) 2)))
      (Rendering|Material|SetScalarParameterValue _asmaterial_instance_dynamic "Percent Out" _bounce :!class /Script/Engine.MaterialInstanceDynamic)
      ;[1 1 1] Add points to score
      (Default|AddPointstoScore (.AsGame%20Mode%20BP (Utilities|Casting|CastToGameMode_BP (Game|GetGameMode))) 2e+01))))

(event EventTick
  (params (DeltaSeconds :type Float%20%28single-precision%29)))

(fn ConstructionScript
  (Rendering|Material|CreateDynamicMaterialInstance (Variables|Default|GetStaticMesh) 2 0 :!class /Script/Engine.PrimitiveComponent))