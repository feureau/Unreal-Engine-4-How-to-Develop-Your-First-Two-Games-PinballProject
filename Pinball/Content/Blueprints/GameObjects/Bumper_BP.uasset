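; Pinball pop bumper actor that knocks an overlapping BallSphere_BP away and awards points.
; On overlap it plays a hit sound, adds score through GameMode_BP and applies an impulse along the bumper-to-ball direction, scaled by DeflectionImpulsePower.
; A timeline drives the mechanism's vertical movement, point light intensity and emissive boost on a dynamic material created in the construction script.
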(event Custom|Bump
  (params (Ball%20Sphere%20BP :type Ball%20Sphere%20BP%20Object%20Reference))
  (Utilities|FlowControl|Sequence
    (:then_0
      ;[1 1 1] Makes sound when bumping ball away
      (Audio|SpawnSoundAttached "/Game/Assets/Sounds/BumperHit_SoundCue.BumperHit_SoundCue" (Variables|Transformation|GetRootComponent)))
    (:then_1
      ;[1 1 1] Add score
      (bind _asgame_mode_bp (Utilities|Casting|CastToGameMode_BP (Game|GetGameMode)))
      (bind _new_score (Default|AddPointstoScore _asgame_mode_bp 1e+01))
      (Development|PrintString (Utilities|String|ToString(Float) _new_score) false false))
    (:then_2
      ;[1 1 1] Bumps ball away
      (Physics|AddImpulse (Variables|/Game/Blueprints/GameObjects/BallSphere_BP.BallSphere_BP_C|GetBallSphere Ball%20Sphere%20BP) (* (Math|Vector|GetUnitDirection(Vector) (Transformation|GetActorLocation) (Transformation|GetActorLocation Ball%20Sphere%20BP)) (Variables|Default|GetDeflection%20Impulse%20Power)) "None" false)
      ;[1 1 1] Light flashes when bumped
      (bind _bumpalpha (Timeline|BumpLerp_Timeline PlayFromStart)
        (:Update
          (Transformation|SetRelativeLocation (Variables|Default|GetSM_PopBumperMechanism) (Math|Vector|Lerp(Vector) "0, 0, 0" "0, 0,-70.000000" _bumpalpha) false false)
          (Rendering|Components|Light|SetIntensity (Variables|Default|GetPointLight) (Math|Float|Lerp 0.0 5e+04 _bumpalpha))
          (Rendering|Material|SetScalarParameterValue (Variables|Default|GetBumperTop_DynamicMaterialInstance) "Emissive Boost" (Math|Float|Lerp 0.0 75.0 _bumpalpha) :!class /Script/Engine.MaterialInstanceDynamic))))))

(event Collision|EventActorBeginOverlap
  (params (OtherActor :type Actor%20Object%20Reference))
  (bind _asball_sphere_bp (Utilities|Casting|CastToBallSphere_BP OtherActor))
  (CallFunction|Bump _asball_sphere_bp))

(fn ConstructionScript
  ;[1 1 1] Create dynamic material instance from SM Pop Bumper Base Material and set it to a variable
  (bind _returnvalue (Rendering|Material|CreateDynamicMaterialInstance (Variables|Default|GetSM_PopBumperBase) 1 0 :!class /Script/Engine.PrimitiveComponent))
  (Variables|Default|SetBumperTop_DynamicMaterialInstance _returnvalue))