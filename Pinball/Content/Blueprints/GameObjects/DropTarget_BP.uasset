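; Drop target, likely for a pinball table, that sinks when hit and shows a configurable letter set in the construction script.
; A hit triggers Drop, which disables mesh collision, quickly slides the mesh down and plays a bumper sound, then fires the OnDrop dispatcher.
; It binds to the game mode's OnGameReset on BeginPlay, and ResetTarget restores the mesh's position and collision.
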(event Custom|Drop
  ;[1 1 1] Move DropTarget down and play hit sound
  (Collision|SetCollisionEnabled (Variables|Default|GetDropTarget_Mesh) "NoCollision") ; so that it doesn't hit anything and does weird things
  (Components|MoveComponentTo (Variables|Default|GetDropTarget_Mesh) "0, 0,-110.000000" "0, 0, 0" false false 0.1 false)
  (Audio|PlaySoundatLocation "/Game/Assets/Sounds/BumperHit_SoundCue.BumperHit_SoundCue" (Transformation|GetActorLocation)))

(event Custom|Reset%20Target
  ;[1 1 1] Reset DropTarget to original position
  (Components|MoveComponentTo 0 "0, 0, 0" "0, 0, 0" false false 0.2 false)
  (Collision|SetCollisionEnabled (Variables|Default|GetDropTarget_Mesh) "QueryAndPhysics"))

(event EventBeginPlay
  (EventDispatchers|BindEventtoOnGameReset (.AsGame%20Mode%20BP (Utilities|Casting|CastToGameMode_BP (Game|GetGameMode))) (EventDispatchers|CreateEvent :!event Custom|Reset%20Target)))

(event Collision|EventActorBeginOverlap
  (params (OtherActor :type Actor%20Object%20Reference)))

(event EventTick
  (params (DeltaSeconds :type Float%20%28single-precision%29)))

(event Collision|EventHit
  (params (MyComp :type Primitive%20Component%20Object%20Reference) (Other :type Actor%20Object%20Reference) (OtherComp :type Primitive%20Component%20Object%20Reference) (bSelfMoved :type Boolean) (HitLocation :type Vector :default "0, 0, 0") (HitNormal :type Vector :default "0, 0, 0") (NormalImpulse :type Vector :default "0, 0, 0") (Hit :type Hit%20Result%20Structure%20%28by%20ref%29))
  ;[1 1 1] If thing gets hit, call drop event and pass to OnDrop event gespacho
  (CallFunction|Drop)
  (Default|CallOnDrop))

(fn ConstructionScript
  (Rendering|Components|TextRender|SetText (Variables|Default|GetU_TextRender) (Utilities|Text|ToText(String) (Variables|Default|GetDropLetter))))