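; VariableBand_BP is a placeable band strung between two posts, sized from an editable Post 2 location.
; The construction script rotates Post1 toward that location, then spawns a matching Post2 mesh there facing back.
; It also adds the SM_BandExtender mesh at Post1's transform, scaling X by the distance between posts while keeping Post1's Y and Z scale.
; All logic runs at construction; the event graph is unused.
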(event EventBeginPlay)

(event Collision|EventActorBeginOverlap
  (params (OtherActor :type Actor%20Object%20Reference)))

(event EventTick
  (params (DeltaSeconds :type Float%20%28single-precision%29)))

(fn ConstructionScript
  (bind _post_1 (Variables|Default|GetPost%201))
  (bind _post_1_2 (Variables|Default|GetPost%201))
  (bind _returnvalue (Transformation|GetRelativeTransform _post_1))
  (bind _scale (Math|Transform|BreakTransform _returnvalue))
  (Utilities|FlowControl|Sequence
    (:then_0
      ;[1 1 1] Make Post1 look at Post 2 Location
      (Transformation|SetRelativeRotation _post_1_2 (Math|Rotator|FindLookatRotation (Variables|/Script/Engine.SceneComponent|GetRelativeLocation _post_1_2) (Variables|Default|GetPost%202%20Location)) false false))
    (:then_1
      ;[1 1 1] Add static mesh componet at Post 2 Location and have it look towards Post1
      (bind _returnvalue_2 (AddComponent|AddStaticMeshComponent false (Math|Transform|MakeTransform (Variables|Default|GetPost%202%20Location) (Math|Rotator|FindLookatRotation (Variables|Default|GetPost%202%20Location) (Variables|/Script/Engine.SceneComponent|GetRelativeLocation (Variables|Default|GetPost%201))) "1,1,1")))
      (bind _output_get (Variables|Default|SetPost%202 _returnvalue_2))
      (Components|StaticMesh|SetStaticMesh _output_get (Variables|/Script/Engine.StaticMeshComponent|GetStaticMesh (Variables|Default|GetPost%201))))
    (:then_2
      ;[1 1 1] Make SM Band Extender scaled to the direction and distance between Post 1 and Post 2 location
      (bind _returnvalue_3 (AddComponent|AddStaticMeshComponent false _returnvalue))
      (Components|StaticMesh|SetStaticMesh _returnvalue_3 "/Game/Assets/StaticMesh/SM_BandExtender.SM_BandExtender")
      (Transformation|SetRelativeScale3D _returnvalue_3 (Math|Vector|MakeVector (/ (Math|Vector|VectorLength (- (Variables|/Script/Engine.SceneComponent|GetRelativeLocation (Variables|Default|GetPost%201)) (Variables|Default|GetPost%202%20Location))) 1e+02) (.y _scale) (.z _scale))))))