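; Rail Blueprint that builds a rail along an editable spline in the construction script, with no active runtime logic.
; It adds one spline mesh component per segment, using a start mesh first, an end mesh last and a mid mesh between.
; Each mesh bends to the local locations and tangents of its two spline points, and the start mesh gets an adjustable start scale on one axis.
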(event EventBeginPlay)

(event Collision|EventActorBeginOverlap
  (params (OtherActor :type Actor%20Object%20Reference)))

(event EventTick
  (params (DeltaSeconds :type Float%20%28single-precision%29)))

(fn ConstructionScript
  (bind _output_get (LocalVariables|SetIndex%20of%20Last%20Spline%20Point (- (Spline|GetNumberOfSplinePoints (Variables|Default|GetSpline)) 2)))
  (for _index (range 0 _output_get)
    ;[1 1 1] If start of spline, add Rail Start Mesh, if end of spline add Rail End Mesh, if mid add Rail Mid Mesh
    (bind _returnvalue (AddComponent|AddSplineMeshComponent false))
    (LocalVariables|SetSpline%20Mesh%20Component _returnvalue)
    (if (== _index 0)
      ;;[1 1 1] Scale multiplier for Rail Start Mesh
      (SplineMesh|SetStartScale (LocalVariables|GetSpline%20Mesh%20Component) (Math|Vector2D|MakeVector2D (Variables|Default|GetInitial%20Scale%20of%20Rail%20Start%20Mesh) 1.0) true :!class /Script/Engine.SplineMeshComponent)
      (Components|StaticMesh|SetStaticMesh (LocalVariables|GetSpline%20Mesh%20Component) (Variables|Default|GetRail%20Start%20Mesh))
      (elif (== _index (LocalVariables|GetIndex%20of%20Last%20Spline%20Point))
        (Components|StaticMesh|SetStaticMesh (LocalVariables|GetSpline%20Mesh%20Component) (Variables|Default|GetRail%20End%20Mesh))
        (else
          (Components|StaticMesh|SetStaticMesh (LocalVariables|GetSpline%20Mesh%20Component) (Variables|Default|GetRail%20Mid%20Mesh)))))
    ;[1 1 1] Spline start and end points
    (SplineMesh|SetStartandEnd (LocalVariables|GetSpline%20Mesh%20Component) (.Location (Spline|GetLocationandTangentatSplinePoint (Variables|Default|GetSpline) _index "Local")) (.Tangent (Spline|GetLocationandTangentatSplinePoint (Variables|Default|GetSpline) _index "Local")) (.Location (Spline|GetLocationandTangentatSplinePoint (Variables|Default|GetSpline) (+ _index 1) "Local")) (.Tangent (Spline|GetLocationandTangentatSplinePoint (Variables|Default|GetSpline) (+ _index 1) "Local")) true :!class /Script/Engine.SplineMeshComponent)))