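; A force zone that steers physics balls passing through it along the direction of its Arrow component.
; Every Tick it gets overlapping BallSphere_BP actors and converts each velocity into the arrow's local space.
; It interpolates that velocity toward a forward-only target with clamped speed, damping sideways motion and enforcing a minimum push.
; The result returns to world space and overrides the ball's linear physics velocity.
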(event EventBeginPlay)

(event Collision|EventActorBeginOverlap
  (params (OtherActor :type Actor%20Object%20Reference)))

(event EventTick
  (params (DeltaSeconds :type Float%20%28single-precision%29))
  (for _array_element (Collision|GetOverlappingActors "/Game/Blueprints/GameObjects/BallSphere_BP.BallSphere_BP_C" :!class /Script/Engine.Actor)
    (Physics|SetPhysicsLinearVelocity (Variables|/Game/Blueprints/GameObjects/BallSphere_BP.BallSphere_BP_C|GetBallSphere (.AsBall%20Sphere%20BP (Utilities|Casting|CastToBallSphere_BP _array_element))) (Math|Transform|TransformDirection (Transformation|GetWorldTransform (Variables|Default|GetArrow)) (Math|Interpolation|VInterpTo (Math|Transform|InverseTransformDirection (Transformation|GetWorldTransform (Variables|Default|GetArrow)) (Transformation|GetVelocity _array_element)) (Math|Vector|MakeVector (Math|Float|Clamp(Float) (.X (Math|Vector|BreakVector (Math|Transform|InverseTransformDirection (Transformation|GetWorldTransform (Variables|Default|GetArrow)) (Transformation|GetVelocity _array_element)))) 8e+02 1.9e+04) 0.0 0.0) (Utilities|Time|GetWorldDeltaSeconds) 15.0)) false "None")))

(fn ConstructionScript)