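; Pinball-style plunger actor that pulls its mesh back while charging and snaps it forward on release.
; ChargePlunger plays a timeline that lerps the mesh's relative location along local Y.
; StopCharge halts the timeline and uses MoveComponentTo to return the mesh quickly to its origin.
; GetBallSpawnLocation converts the local BallLocation to world space through the actor transform for ball spawning.
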(event Custom|Charge%20Plunger
  ;[1 1 1] Slowly pull plunger-staticmesh back
  (bind _charge_alpha (Timeline|Charge%20Timeline PlayFromStart)
    (:Update
      (Transformation|SetRelativeLocation (Variables|Default|GetPlunger_StaticMesh) (Math|Vector|Lerp(Vector) "0, 0, 0" "0,150.000000, 0" _charge_alpha) false false))))

(event Custom|Stop%20Charge
  ;[1 1 1] Fires plunger staticmesh back to its original location
  (Utilities|FlowControl|Sequence
    (:then_0
      ;[1 1 1] Slowly pull plunger-staticmesh back
      (bind _charge_alpha (Timeline|Charge%20Timeline Stop)
        (:Update
          (Transformation|SetRelativeLocation (Variables|Default|GetPlunger_StaticMesh) (Math|Vector|Lerp(Vector) "0, 0, 0" "0,150.000000, 0" _charge_alpha) false false))))
    (:then_1
      (Components|MoveComponentTo (Variables|Default|GetPlunger_StaticMesh) "0, 0, 0" "0, 0, 0" false false 0.1 false))))

(fn ConstructionScript)

(fn GetBallSpawnLocation
  (bind _returnvalue (Transformation|GetActorTransform))
  (bind _ball_location (Variables|Default|GetBall%20Location))
  (bind _returnvalue_2 (Math|Transform|TransformLocation _returnvalue _ball_location))
  ;[1 1 1] Converts Local Transform location of "Ball Location" in relation to "GetActorLocation"to World Transform
  (Development|PrintString (Utilities|String|BuildString(Object) "Ball location " (Utilities|String|ToString(Vector) _returnvalue_2) 0 " end") false false "(R=0.000000,G=0.660000,B=1.000000,A=1.000000)" 5.0)
  (return _returnvalue_2))