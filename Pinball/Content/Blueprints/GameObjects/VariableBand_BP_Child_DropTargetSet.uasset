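; Variable band child that adds a row of lettered drop targets and raises the game mode's multiplier when its target counter runs out.
; The construction script uppercases the target string and spawns one DropTarget_BP child actor per letter, evenly spaced between the band's two posts and offset sideways.
; It binds to each target's drop event and the game mode's reset event, with handlers for counting down and restoring the counter to the string length.
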(event Custom|Process%20Drop%20Targets
  ;[1 1 1] If Target Counter reaches 0
  (bind _result (Math|Integer|DecrementInt (Variables|Default|GetTargetCounter))
    (:%20%20
      (if (== _result 0)
        ;[1 1 1] increase multiplier in the game mode
        (Math|Float|IncrementFloat (Variables|/Game/Blueprints/GameMode_BP.GameMode_BP_C|GetMultiplier (.AsGame%20Mode%20BP (Utilities|Casting|CastToGameMode_BP (Game|GetGameMode)))))))))

(event Custom|Reset%20Drop%20Target%20Counter
  ;[1 1 1] Set Target Counter to length of Drop Target String
  (Variables|Default|SetTargetCounter (Utilities|String|Len (Variables|Default|GetDropTargetString))))

(event EventBeginPlay
  (|CallParentFunction)
  (EventDispatchers|BindEventtoOnGameReset (.AsGame%20Mode%20BP (Utilities|Casting|CastToGameMode_BP (Game|GetGameMode))) (EventDispatchers|CreateEvent :!event Custom|Reset%20Drop%20Target%20Counter)))

(event Collision|EventActorBeginOverlap
  (params (OtherActor :type Actor%20Object%20Reference))
  (|CallParentFunction OtherActor) ; This node is disabled and will not be called.\nDrag off pins to build functionality.
)

(event EventTick
  (params (DeltaSeconds :type Float%20%28single-precision%29))
  (|CallParentFunction DeltaSeconds) ; This node is disabled and will not be called.\nDrag off pins to build functionality.
)

(fn ConstructionScript
  (|CallParentFunction)
  (bind _output_get (Variables|Default|SetDropTargetString (Class|KismetStringLibrary|ToUpper (Variables|Default|GetDropTargetString))))
  (for (_array_element _array_index) (Utilities|String|GetCharacterArrayfromString _output_get)
    (LocalVariables|SetCurrent%20Letter _array_element)
    (bind _returnvalue (AddComponent|AddChildActorComponent false (Math|Transform|MakeTransform (+ (* (Math|Vector|GetForwardVector (Variables|Default|GetPost%201)) (* (+ _array_index 1) (/ (Math|Vector|VectorLength (- (Variables|/Script/Engine.SceneComponent|GetRelativeLocation (Variables|Default|GetPost%201)) (Variables|/Script/Engine.SceneComponent|GetRelativeLocation (Variables|Default|GetPost%202)))) (Math|Conversions|ToFloat(Integer) (+ (Utilities|Array|Length (Utilities|String|GetCharacterArrayfromString _output_get)) 1))))) (* (Math|Vector|GetRightVector (Variables|Default|GetPost%201)) 2e+01)) (Variables|/Script/Engine.SceneComponent|GetRelativeRotation (Variables|Default|GetPost%201)) "1,1,1")))
    ;[1 1 1] Set character to the letter thingy on the tiles
    (bind _asdrop_target_bp (Utilities|Casting|CastToDropTarget_BP (Variables|/Script/Engine.ChildActorComponent|GetChildActor _returnvalue)))
    (bind _output_get_2 (Variables|/Game/Blueprints/GameObjects/DropTarget_BP.DropTarget_BP_C|SetDropLetter _asdrop_target_bp (LocalVariables|GetCurrent%20Letter)))
    (Rendering|Components|TextRender|SetText (Variables|/Game/Blueprints/GameObjects/DropTarget_BP.DropTarget_BP_C|GetU_TextRender _asdrop_target_bp) (Utilities|Text|ToText(String) _output_get_2))
    (EventDispatchers|BindEventtoOnDrop _asdrop_target_bp (EventDispatchers|CreateEvent :!event Custom|Process%20Drop%20Targets))))