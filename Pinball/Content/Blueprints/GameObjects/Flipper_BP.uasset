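; Flipper actor, configurable as a left or right flipper, that swings between two rotations on Flip and Flop events.
; The construction script sets start and end rotations from FlipType, applies the start pose and mirrors the right variant with negative X scale.
; Flip and Flop use MoveComponentTo to rotate the root in place, each with its own duration.
; A delayed Flip/Flop test chain is left disconnected.
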(event Custom|Flop
  (Components|MoveComponentTo (Variables|Transformation|GetRootComponent) (Transformation|GetActorLocation) (Variables|Default|GetStart%20Rotation) false false (Variables|Default|GetTime%20to%20complete%20a%20Flop) false))

(event Custom|Flip
  (Components|MoveComponentTo (Variables|Transformation|GetRootComponent) (Transformation|GetActorLocation) (Variables|Default|GetEnd%20Rotation) false false (Variables|Default|GetTime%20to%20complete%20a%20Flip) false))

(event EventBeginPlay)

(event Collision|EventActorBeginOverlap
  (params (OtherActor :type Actor%20Object%20Reference)))

(event EventTick
  (params (DeltaSeconds :type Float%20%28single-precision%29)))

(fn ConstructionScript
  ;[1 1 1] Set start and end rotation variables depending on left or right flip type position
  (Variables|Default|SetStart%20Rotation (Utilities|Select :Index (Variables|Default|GetFlipType) :NewEnumerator0 "0,20.000000, 0" :NewEnumerator1 "0.000000,-20.000000, 0"))
  (Variables|Default|SetEnd%20Rotation (Utilities|Select :Index (Variables|Default|GetFlipType) :NewEnumerator0 "0,-20.000000, 0" :NewEnumerator1 "0.000000,20.000000,0.000000"))
  (Transformation|SetRelativeRotation (Variables|Transformation|GetRootComponent) (Variables|Default|GetStart%20Rotation) false false)
  ;[1 1 1] Make flipper flipped for right or left position depending on flipper type enum selection
  (switch Utilities|FlowControl|Switch|SwitchonFlipperType_Enum (Variables|Default|GetFlipType)
    (:NewEnumerator0
      (Transformation|SetRelativeScale3D (Variables|Transformation|GetRootComponent) "1.000000,1.000000,1.000000"))
    (:NewEnumerator1
      (Transformation|SetRelativeScale3D (Variables|Transformation|GetRootComponent) "-1.000000,1.000000,1.000000"))))