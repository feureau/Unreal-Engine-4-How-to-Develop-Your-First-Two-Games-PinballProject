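; BallSphere_BP is the pinball ball actor, moving a physics sphere across the table with simulated gravity and rolling audio.
; Each tick it applies a fake gravity acceleration along the table, scaled by delta time.
; A downward line trace finds the surface normal, and a small impulse against it keeps the ball stuck to the table.
; Rolling sound volume and pitch follow ball speed, and a loose-ball sound plays attached on BeginPlay.
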(event EventBeginPlay
  (Audio|SpawnSoundAttached "/Game/Assets/Sounds/Pinball_BallLoose_Cue.Pinball_BallLoose_Cue" (Variables|Default|GetBallSphere)))

(event Collision|EventActorBeginOverlap
  (params (OtherActor :type Actor%20Object%20Reference)))

(event EventTick
  (params (DeltaSeconds :type Float%20%28single-precision%29))
  (bind _returnvalue (Transformation|GetActorLocation))
  (bind _returnvalue_2 (Transformation|GetVelocity))
  (bind _returnvalue_3 (Math|Vector|VectorLength _returnvalue_2))
  (bind _returnvalue_4 (/ _returnvalue_3 1e+03))
  (Utilities|FlowControl|Sequence
    (:then_0
      ;[1 1 1] Fake Gravity. Add force towards Y axis as set in gravitational impulse speed
      (Physics|AddForce (Variables|Default|GetBallSphere) (* (Variables|Default|GetGravitational%20impulse%20speed) (Utilities|Time|GetWorldDeltaSeconds)) "None" true))
    (:then_1
      ;[1 1 1] Impulse ball to the direction of table
      (bind _outhit (Collision|LineTraceByChannel _returnvalue (- _returnvalue (Math|Vector|MakeVector 0.0 0.0 5e+02)) "TraceTypeQuery1" false 0 "None"))
      (Physics|AddImpulse (Variables|Default|GetBallSphere) (* (* (.impactnormal _outhit) -1.0) (* (Variables|Default|GetStickyness%20To%20Table%20Factor) (Utilities|Time|GetWorldDeltaSeconds))) "None" false))
    (:then_2
      (Audio|Components|Audio|SetVolumeMultiplier (Variables|Default|GetBallRollingSound) (Math|Float|Clamp(Float) _returnvalue_4) :!class /Script/Engine.AudioComponent)
      (Audio|Components|Audio|SetPitchMultiplier (Variables|Default|GetBallRollingSound) (Math|Float|Clamp(Float) _returnvalue_4 0.97 1.2)))))

(fn ConstructionScript)