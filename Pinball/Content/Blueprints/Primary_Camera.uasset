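; Primary camera that adapts its field of view to the viewport aspect ratio at BeginPlay, starting from a default horizontal FOV set in the construction script.
; On viewports wider than the reference ratio, it scales that FOV linearly to a vertical value, then converts it to horizontal with a tan/atan formula using the current ratio.
; Otherwise it keeps the default; an aspect ratio and FOV debug print is switched off.
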(event EventBeginPlay
  (Variables|Default|SetDefault%20Aspect%20Ratio (/ (Variables|Default|GetHorizontal%20Aspect%20Ratio) (Variables|Default|GetVertical%20Aspect%20Ratio)))
  (if (> (Utilities|GetCurrentAspectRatio) (Variables|Default|GetDefault%20Aspect%20Ratio)) ; If current viewport aspect ratio is \nwider than default aspect ratio,\nthen calculate and set HFOV based on VFOV\nOtherwise revert to default Horizontal FOV
    ;[1 1 1] Calculate and set HFOV based on VFOV
    (bind _output_get (Variables|/Script/Engine.CameraComponent|SetFieldOfView (Variables|CameraActor|GetCameraComponent) (Utilities|TANdAtanConverter (/ (* (Variables|Default|GetDefault%20Desired%20Horizontal%20FOV) (Variables|Default|GetVertical%20Aspect%20Ratio)) (Variables|Default|GetHorizontal%20Aspect%20Ratio)))))
    (Utilities|PrintAspectRatio,HFOV,andVFOV (Utilities|TANdAtanConverter (/ (* _output_get (Variables|Default|GetVertical%20Aspect%20Ratio)) (Variables|Default|GetHorizontal%20Aspect%20Ratio))) _output_get false)
    (else
      ;[1 1 1] Revert to default desired horizontal FOV
      (bind _output_get_2 (Variables|/Script/Engine.CameraComponent|SetFieldOfView (Variables|CameraActor|GetCameraComponent) (Variables|Default|GetDefault%20Desired%20Horizontal%20FOV)))
      (Utilities|PrintAspectRatio,HFOV,andVFOV (Utilities|TANdAtanConverter (/ (* _output_get_2 (Variables|Default|GetVertical%20Aspect%20Ratio)) (Variables|Default|GetHorizontal%20Aspect%20Ratio))) _output_get_2 false))))

(fn ConstructionScript
  (Camera|SetFieldOfView (Variables|CameraActor|GetCameraComponent) (Variables|Default|GetDefault%20Desired%20Horizontal%20FOV)))