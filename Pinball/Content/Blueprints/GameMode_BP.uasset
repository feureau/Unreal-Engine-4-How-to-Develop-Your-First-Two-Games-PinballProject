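; Pinball game mode that runs the game from main menu through ball play to high-score entry, tracking score, multiplier and balls remaining.
; ResetGame restores class defaults, shows the HUD and spawns a ball at the plunger; each ball's OnDestroyed spawns another or ends the game.
; EndGame opens high-score entry, then returns to the menu if saved scores exist and the lowest isn't beaten.
; GetSavegameData lazily loads or creates, sorts and caches the save.
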(event Custom|Reset%20Game
  (bind _returnvalue (Game|GetPlayerController 0))
  (bind (_score _multiplier _ballsremaining) (Utilities|GetClassDefaults "GameMode_BP_C"))
  (bind _asplayer_controller_bp (Utilities|Casting|CastToPlayerController_BP _returnvalue))
  ;[1 1 1] Reset all variable values to default
  (Variables|Default|SetScore _score)
  (Variables|Default|SetMultiplier _multiplier)
  (Variables|Default|SetBallsRemaining _ballsremaining)
  (CallFunction|SpawnBall)
  (Default|CreatePlayerHUD _asplayer_controller_bp)
  (Variables|/Script/Engine.PlayerController|SetbShowMouseCursor _asplayer_controller_bp false))

(event Custom|Create%20Main%20Menu
  (bind _returnvalue (Game|GetPlayerController 0))
  (bind _asplayer_controller_bp (Utilities|Casting|CastToPlayerController_BP _returnvalue))
  ;[1 1 1] Display MainMenu_WidgetBP to viewport and show mouse cursor
  (Viewport|RemoveAllWidgets)
  (bind _returnvalue_2 (UserInterface|CreateWidget "/Game/Blueprints/Widgets/MainMenu_WidgetBP.MainMenu_WidgetBP_C" _asplayer_controller_bp))
  (UserInterface|Viewport|AddtoViewport _returnvalue_2 0)
  (Variables|/Script/Engine.PlayerController|SetbShowMouseCursor _asplayer_controller_bp true))

(event Custom|SpawnBall
  ;[1 1 1] Spawn ball sphere bp
  (bind _outactors (Actor|GetAllActorsOfClass "/Game/Blueprints/Plunger_BP.Plunger_BP_C"))
  (bind _returnvalue (Game|SpawnActorfromClass "/Game/Blueprints/BallSphere_BP.BallSphere_BP_C" (Math|Transform|MakeTransform (Default|GetBallSpawnLocation (Utilities|Array|Get(acopy) _outactors)) "0, 0, 0" "1,1,1") "Undefined" 0 0))
  ;[1 1 1] If ball destroyed, check if player still has balls remaining to play, if true, spawn, else end game.
  (Game|BindEventtoOnDestroyed _returnvalue (delegate Custom|OnBallDestroyed)))

(event Custom|EndGame
  (CallFunction|CreateHighscoresList)
  ;[1 1 1] Save game data
  (bind _current_save_object (CallFunction|GetSavegameData))
  (if (not (<= (Utilities|Array|Length (Variables|/Game/Blueprints/HighScoreSave_BP.HighScoreSave_BP_C|GetSaveStruct _current_save_object)) 0))
    (bind _lowest_score_struct (Default|DetermineLowestValueScore _current_save_object))
    (if (< (.score _lowest_score_struct) (Variables|Default|GetScore))
      ;[1 1 1] Player achieves high score
      (CallFunction|CreateHighscoresList)
      (else
        ;[1 1 1] Player did not achieve high score
        (CallFunction|CreateMainMenu)))))

(event Custom|OnBallDestroyed
  (params (DestroyedActor :type Actor%20Object%20Reference))
  ;[1 1 1] If ball destroyed, check if player still has balls remaining to play, if true, spawn, else end game.
  (if (> (Variables|Default|GetBallsRemaining) 0)
    (CallFunction|SpawnBall)
    (Math|Integer|DecrementInt (Variables|Default|GetBallsRemaining))
    (else
      (CallFunction|EndGame))))

(event Custom|Create%20Highscores%20List
  (bind _returnvalue (Game|GetPlayerController 0))
  (bind _asplayer_controller_bp (Utilities|Casting|CastToPlayerController_BP _returnvalue))
  ;[1 1 1] Display highscore entry bp widget to viewport and show mouse cursor
  (bind _returnvalue_2 (UserInterface|CreateWidget "/Game/Blueprints/Widgets/HighScoreEntry_WidgetBP.HighScoreEntry_WidgetBP_C" _asplayer_controller_bp))
  (UserInterface|Viewport|AddtoViewport _returnvalue_2 0)
  (Variables|/Script/Engine.PlayerController|SetbShowMouseCursor _asplayer_controller_bp true))

(event EventBeginPlay
  (CallFunction|CreateMainMenu))

(event EventTick
  (params (DeltaSeconds :type Float%20%28single-precision%29)))

(fn ConstructionScript)

(fn AddHighScore
  (params (Points%20to%20add :type Float%20%28single-precision%29))
  (bind _output_get (Variables|Default|SetScore (+ (Variables|Default|GetScore) (* Points%20to%20add (Variables|Default|GetMultiplier)))))
  (return _output_get))

(fn GetSavegameData
  (bind _currentsaveobject (Variables|Default|GetCurrentSaveObject)
    (:then
      (return _currentsaveobject))
    (:else
      (bind _returnvalue (SaveGame|DoesSaveGameExist (Variables|Default|GetHigh%20Score%20Save%20Name)))
      (if _returnvalue
        (bind _returnvalue_2 (SaveGame|LoadGamefromSlot (Variables|Default|GetHigh%20Score%20Save%20Name)))
        (bind _ashigh_score_save_bp (Utilities|Casting|CastToHighScoreSave_BP _returnvalue_2)
          (:then
            (Default|SortSavedData _ashigh_score_save_bp)
            (bind _output_get (Variables|Default|SetCurrentSaveObject _ashigh_score_save_bp))
            (return _output_get))
          (:CastFailed
            (return 0)))
        (else
          (bind _returnvalue_3 (SaveGame|CreateSaveGameObject "/Game/Blueprints/HighScoreSave_BP.HighScoreSave_BP_C"))
          (bind _ashigh_score_save_bp_2 (Utilities|Casting|CastToHighScoreSave_BP _returnvalue_3)
            (:then
              (Default|SortSavedData _ashigh_score_save_bp_2)
              (bind _output_get_2 (Variables|Default|SetCurrentSaveObject _ashigh_score_save_bp_2))
              (return _output_get_2))
            (:CastFailed
              (return 0))))))))