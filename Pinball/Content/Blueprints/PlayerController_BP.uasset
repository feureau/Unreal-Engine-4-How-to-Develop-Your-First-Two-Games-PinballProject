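; Player controller for a pinball game that routes input to the table's flippers and plunger and creates the HUD.
; On BeginPlay it finds every flipper actor, sorting each into a left or right array by its flip type, and keeps the first plunger found.
; Left and right inputs flip and flop all flippers on that side, while the charge input starts and stops the plunger's charge.
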(event Custom|Detect%20Flippers
  ;[1 1 1] Find all flippers and add them to left or right flippers arrays
  (bind _outactors (Actor|GetAllActorsOfClass "/Game/Blueprints/Flipper_BP.Flipper_BP_C"))
  (for _array_element _outactors
    (Utilities|Array|Add (Utilities|Select :Index (Variables|/Game/Blueprints/Flipper_BP.Flipper_BP_C|GetFlipType _array_element) :NewEnumerator0 (Variables|Default|GetLeft%20Flippers) :NewEnumerator1 (Variables|Default|GetRight%20Flippers)) _array_element)))

(event Custom|CreatePlayerHUD
  (Viewport|RemoveAllWidgets)
  (bind _returnvalue (UserInterface|CreateWidget "/Game/Blueprints/Widgets/PinballHUD_WidgetBP.PinballHUD_WidgetBP_C"))
  (UserInterface|Viewport|AddtoViewport _returnvalue 0))

(event Custom|Detect%20Plungers
  ;[1 1 1] Find all in class plunger - set the first one to Plunger variable
  (bind _outactors (Actor|GetAllActorsOfClass "/Game/Blueprints/Plunger_BP.Plunger_BP_C"))
  (if (> (Utilities|Array|Length _outactors) 0)
    (Variables|Default|SetPlunger (Utilities|Array|Get(acopy) _outactors))))

(event EventBeginPlay
  (CallFunction|DetectFlippers)
  (CallFunction|DetectPlungers)
  (CallFunction|CreatePlayerHUD))

(event Input|ActionEvents|InputActionLeftFlipper
  (params (Key :type Key%20Structure))
  ;[1 1 1] Trigger and release left flipper
  (:Pressed
    (for _array_element (Variables|Default|GetLeft%20Flippers)
      (Default|Flip _array_element)))
  (:Released
    (for _array_element_2 (Variables|Default|GetLeft%20Flippers)
      (Default|Flop _array_element_2))))

(event Input|ActionEvents|InputActionRightFlipper
  (params (Key :type Key%20Structure))
  ;[1 1 1] Trigger and release right flipper
  (:Pressed
    (for _array_element (Variables|Default|GetRight%20Flippers)
      (Default|Flip _array_element)))
  (:Released
    (for _array_element_2 (Variables|Default|GetRight%20Flippers)
      (Default|Flop _array_element_2))))

(event Input|ActionEvents|InputActionChargePlunger
  (params (Key :type Key%20Structure))
  ;[1 1 1] Charge and stop charge plunger
  (:Pressed
    (Default|ChargePlunger (Variables|Default|GetPlunger)))
  (:Released
    (Default|StopCharge (Variables|Default|GetPlunger))))

(fn ConstructionScript)