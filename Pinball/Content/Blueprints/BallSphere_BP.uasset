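; BallSphere_BP is a physics-driven ball that is pushed along and kept pressed against the table surface beneath it.
; Each Tick applies a DefaultSpeed impulse to BallSphere, scaled by delta time.
; A downward Visibility line trace, debug-drawn each frame, finds the surface normal, and a second impulse along its inverse, scaled by StickynessToTableFactor and delta time, sticks the ball to that surface.
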(event EventBeginPlay)

(event Collision|EventActorBeginOverlap
  (params (OtherActor :type Actor%20Object%20Reference)))

(event EventTick
  (params (DeltaSeconds :type Float%20%28single-precision%29))
  (bind _returnvalue (Transformation|GetActorLocation))
  (Physics|AddImpulse (Variables|Default|GetBallSphere) (* (Variables|Default|GetDefault%20Speed) DeltaSeconds) "None" false)
  (bind _outhit (Collision|LineTraceByChannel _returnvalue (- _returnvalue "0, 0,500.000000") "TraceTypeQuery1" false 0 "ForOneFrame"))
  (Physics|AddImpulse (Variables|Default|GetBallSphere) (* (* (.impactnormal _outhit) -1.0) (* (Variables|Default|GetStickyness%20To%20Table%20Factor) (Utilities|Time|GetWorldDeltaSeconds))) "None" false))

(fn ConstructionScript)